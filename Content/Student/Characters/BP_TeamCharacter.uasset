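; Team-aware player character Blueprint that tints its armour to match the team it belongs to.
; SetTeam stores the team, selects ArmourColour (black for none, blue or red for the two teams) and calls SetupMaterial; GetTeam exposes the value.
; Init disables shadow casting on the WeaponWidget component and binds its PlayerWeaponUI to this character before running the parent Init.
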(event EventBeginPlay)

(event Collision|EventActorBeginOverlap
  (params (OtherActor :type Actor%20Object%20Reference)))

(event EventTick
  (params (DeltaSeconds :type Float%20%28single-precision%29))
  (|CallParentFunction DeltaSeconds) ; This node is disabled and will not be called.\nDrag off pins to build functionality.
)

(event EventSetTeam
  (params (Team :type teamsList%20Enum :default "NewEnumerator0"))
  (bind _output_get (Variables|Default|SetTeam Team))
  (Variables|Default|SetArmourColour (Utilities|Select :Index _output_get :NewEnumerator0 "" :NewEnumerator1 "(R=0.000000,G=0.089579,B=1.000000,A=1.000000)" :NewEnumerator2 "(R=1.000000,G=0.020315,B=0.000000,A=1.000000)"))
  (CallFunction|SetupMaterial))

(fn ConstructionScript
  (|CallParentFunction))

(fn Init
  (Rendering|SetCastShadow (Variables|Default|GetWeaponWidget) false)
  (Default|Init (.AsPlayer%20Weapon%20UI (Utilities|Casting|CastToPlayerWeaponUI (UserInterface|GetUserWidgetObject (Variables|Default|GetWeaponWidget)))) self)
  (|CallParentFunction))

(fn GetTeam
  (return (Variables|Default|GetTeam)))