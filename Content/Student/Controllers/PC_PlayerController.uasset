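; Player controller for team game modes (BP and CTF) that stores the player's team and handles respawning after death.
; Each mode's init event caches its game mode and binds to the controlled character's death event through a message interface.
; On death, the view blends to that mode's spectator camera, then after a short delay the game mode is messaged to respawn a team character.
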(event Custom|CharacterDestroyed
  (params (DeadCharacter :type BP%20Base%20Character%20Object%20Reference) (Killer :type Actor%20Object%20Reference))
  (Game|Player|SetViewTargetwithBlend (Default|GetSpecCam (Variables|Default|GetgmCTF)) 0.0 "VTBlend_Linear" 0.0 false)
  (Utilities|FlowControl|Delay 1.0)
  (Class|BpiGamemode|GmRespawn(Message) (Game|GetGameMode) self (Variables|Default|GetTeam) "/Game/Student/Characters/BP_TeamCharacter.BP_TeamCharacter_C"))

(event Custom|CharacterWasDestroyed
  (params (DeadCharacter :type BP%20Base%20Character%20Object%20Reference) (Killer :type Actor%20Object%20Reference))
  (Game|Player|SetViewTargetwithBlend (Default|GetSpecCam (Variables|Default|GetgmBP)) 0.0 "VTBlend_Linear" 0.0 false)
  (Utilities|FlowControl|Delay 1.0)
  (Class|BpiGamemode|GmRespawn(Message) (Game|GetGameMode) self (Variables|Default|GetTeam) "/Game/Student/Characters/BP_TeamCharacter.BP_TeamCharacter_C"))

(event EventSetTeam
  (params (Team :type teamsList%20Enum :default "NewEnumerator0"))
  (bind _output_get (Variables|Default|SetTeam Team))
  (Development|PrintString (Utilities|String|Append "Joined" (Utilities|String|EnumtoString _output_get))))

(event EventInitBP
  (params (gamemode :type BP-Game%20Mode%20Object%20Reference))
  (bind _asbasecharacter (Class|BPIBaseCharacter|BpiBasecharacter(Message) (Pawn|GetControlledPawn)))
  (EventDispatchers|BindEventtoOnDeath _asbasecharacter (delegate Custom|CharacterWasDestroyed))
  (Variables|Default|SetgmBP gamemode))

(event EventInitCTF
  (params (gamemode :type CTF-Game%20Mode%20Object%20Reference))
  (bind _asbasecharacter (Class|BPIBaseCharacter|BpiBasecharacter(Message) (Pawn|GetControlledPawn)))
  (EventDispatchers|BindEventtoOnDeath _asbasecharacter (delegate Custom|CharacterDestroyed))
  (Variables|Default|SetgmCTF gamemode))

(fn ConstructionScript)

(fn CanEndCheck
  (return false))

(fn GetGamemode
  (return 0))

(fn BombPlant
  (return 0))

(fn GetTeam
  (return (Variables|Default|GetTeam)))

(fn Playercontroller
  (return self))